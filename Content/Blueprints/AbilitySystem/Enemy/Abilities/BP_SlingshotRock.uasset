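; BP_SlingshotRock is the rock actor for an enemy slingshot ability, adding a random tumbling spin to its mesh.
; BeginPlay picks independent random yaw, pitch and roll rates in either direction.
; Tick scales these rates by delta time and applies them to RockMesh as local rotation, keeping the spin frame-rate independent.
; The graph holds only this rotation, with no movement or hit logic.
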(event `self.ReceiveBeginPlay`
  (bind _returnvalue (`KismetMathLibrary.RandomFloatInRange` -360.0 360.0))
  (set `self.LocalYarRotationRate` _returnvalue)
  (set `self.LocalPitchRotationRate` _returnvalue)
  (set `self.LocalRollRotationRate` _returnvalue))

(event `self.ReceiveTick`
  (params (DeltaSeconds :type "Float (single-precision)"))
  (`SceneComponent.K2_AddLocalRotation` (`self.RockMesh`) (`KismetMathLibrary.MakeRotator` (* DeltaSeconds (`self.LocalRollRotationRate`)) (* DeltaSeconds (`self.LocalPitchRotationRate`)) (* DeltaSeconds (`self.LocalYarRotationRate`))) false false))

(fn `UserConstructionScript`)