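; Fire Blast ability fireball that flies out like a boomerang and explodes on its way back to ReturnToActor.
; On the server, two chained timelines lerp it to an apex ahead, then back toward that actor's current location.
; Within ExplodeDistance, it calls OnHit, applies radial damage effects to nearby live combatants except its owner, with upward-angled knockback and death impulse, then destroys itself.
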(event `self.StartOutgoingTimeline`
  (bind _explosiondamageparams (`self.ExplosionDamageParams`))
  (bind _array (`|MakeArray` (`self.GetOwner`)))
  (`/Engine/EditorBlueprintResources/ActorMacros.Switch Has Authority`
    (:`Authority`
      ;[1 1 1] 火球飞行
      (set `self.InitialLocation` (`self.K2_GetActorLocation`)) ; 初始位置
      (set `self.ApexLocation` (+ (`self.InitialLocation`) (* (`self.GetActorForwardVector`) (`self.TravelDistance`)))) ; 最远距离
      (bind (_direction _outgoingtrack) (`Timeline|OutgoingTimeline`)
        (:`Update`
          (`self.K2_SetActorLocation` (`KismetMathLibrary.VLerp` (`self.InitialLocation`) (`self.ApexLocation`) _outgoingtrack)) ; 出去
        )
        (:`Finished`
          (bind (_direction_2 _returningtrack) (`Timeline|ReturningTimeline`)
            (:`Update`
              (`self.K2_SetActorLocation` (`KismetMathLibrary.VLerp` (`self.ApexLocation`) (`self.K2_GetActorLocation` (`self.ReturnToActor`)) _returningtrack)) ; 返回
              ;[1 1 1] 火球爆炸
              (if (`self.IsWithinExplodeDistance`)
                (`self.OnHit`)
                ;[1 1 1] 设置伤害参数
                (`AuraAbilitySystemLibrary.SetIsRadialDamageEffectParams` (`self.ExplosionDamageParams`) true 50.0 100.0 (`self.K2_GetActorLocation`))
                ;;[1 1 1] 识别敌人
                (`KismetArrayLibrary.Array_Add` _array self)
                (bind _outoverlappingactors (`AuraAbilitySystemLibrary.GetLivePlayerWithRadius` self _array 300.0 (`self.K2_GetActorLocation`)))
                (set `self.OverlappingPlayers` _outoverlappingactors)
                (for _array_element (`self.OverlappingPlayers`)
                  (`AuraAbilitySystemLibrary.SetEffectParamsTargetASC` _explosiondamageparams (`AbilitySystemBlueprintLibrary.GetAbilitySystemComponent` _array_element))
                  (bind _returnvalue (- (`self.K2_GetActorLocation` _array_element) (`self.K2_GetActorLocation`)))
                  (bind (_returnvalue_roll _returnvalue_pitch _returnvalue_yaw) (`KismetMathLibrary.BreakRotator` (`KismetMathLibrary.MakeRotFromX` _returnvalue)))
                  (`AuraAbilitySystemLibrary.SetKnockbackDirection` _explosiondamageparams (`KismetMathLibrary.GetForwardVector` (`KismetMathLibrary.MakeRotator` _returnvalue_roll 45.0 _returnvalue_yaw)))
                  (`AuraAbilitySystemLibrary.SetDeathImpulseDirection` _explosiondamageparams _returnvalue)
                  (`AuraAbilitySystemLibrary.ApplyDamageEffect` _explosiondamageparams))
                (`self.K2_DestroyActor`)))))))))

(fn `IsWithinExplodeDistance`
  (returns (ReturnValue :type Boolean))
  (return (<= (`KismetMathLibrary.VSize` (- (`self.K2_GetActorLocation`) (`self.K2_GetActorLocation` (`self.ReturnToActor`)))) (`self.ExplodeDistance`))))

(fn `UserConstructionScript`)