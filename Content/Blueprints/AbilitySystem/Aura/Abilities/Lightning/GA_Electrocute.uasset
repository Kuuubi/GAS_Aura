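; Channeled lightning Gameplay Ability that shocks the target under the mouse and chains to additional targets while input is held.
; A montage event locks movement, spawns ShockLoop beam cues and starts a looping timer that commits cost and damages all targets, ending when cost fails.
; Release respects a minimum cast time, then cleanup removes cues, applies an authority-only final damage effect and commits cooldown.
; Target-death events remove chain cues.
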(event `DamageAndCost`
  ;[1 1 1] 应用伤害和成本,冷却
  (bind _returnvalue (`self.K2_CommitAbilityCost` false))
  (if _returnvalue
    (`self.ApplyDamage`)
    (else
      (`self.ClearTimerAndEndAbility`))))

(event `self.K2_ActivateAbility`
  (`self.EnforceImplementsCombatInterface`)
  ;[0.9289 0.6967 1] 保存鼠标命中信息变量
  (bind (_asynctaskproxy _datahandle) (`TargetDataUnderMouse.CreateTargetDataUnderMouse`)
    (:`ValidData`
      (`self.StoreMouseDataInfo` (`AbilitySystemBlueprintLibrary.GetHitResultFromTargetData` _datahandle))
      (`self.StoreOwnerVariables`)
      (`|ExecutionSequence`
        (:`then_0`
          ;[1 1 1] 抬手/持续释放技能动画
          (set `PlayerController.bShowMouseCursor` false (`self.OwnerPlayerController`))
          (`self.UpdateFacingTarget`)
          (`self.K2_ExecuteGameplayCue` (struct :`TagName` "GameplayCue.ShockBurst"))
          (`AbilityTask_PlayMontageAndWait.CreatePlayMontageAndWaitProxy` "None" (`self.Montage_Electrocute`) 1.0 "None" false
            (:`then`
              (`AbilityTask_WaitGameplayEvent.WaitGameplayEvent` (struct :`TagName` "Event.Montage.Electrocute") null true
                (:`EventReceived`
                  (`self.InShockLoop`)
                  ;[1 1 1] 生成闪电
                  (`self.SpawnElectricBeam`)
                  ;[1 1 1] 应用伤害和成本,冷却
                  (bind _returnvalue (`KismetSystemLibrary.K2_SetTimerDelegate` (delegate `DamageAndCost`) (`self.DamageDeltaTime`) true))
                  (set `self.DamageAndCostTimer` _returnvalue))))))
        (:`then_1`
          ;[1 1 1] 技能按键抬起结束
          (bind (_asynctaskproxy_2 _timeheld) (`AbilityTask_WaitInputRelease.WaitInputRelease` false)
            (:`OnRelease`
              (set `self.TimeHeld` _timeheld)
              (if (< (`self.TimeHeld`) (`self.MinSpellTime`))
                (`self.K2_HasAuthority`
                  (:`True`
                    (`KismetSystemLibrary.Delay` (- (`self.MinSpellTime`) (`self.TimeHeld`)))
                    (`self.ClearTimerAndEndAbility` :!label _label))
                  (:`False`
                    (`self.PrepareToEndAbility`)))
                (else
                  (goto _label))))))))))

(event `self.PrimaryTargetDied`
  (params (DeadActor :type "Actor Object Reference"))
  ;[1 0.5176 0.1255] 主要目标敌人死亡
  ;;[1 1 1] 移除闪电链接的全部额外敌人
  (for _array_element (`self. AdditionalTargets`)
    (`self.RemoveShockLoopCuefromAdditionalTarget` _array_element))
  (`BlueprintMapLibrary.Map_Clear` (`self.AdditionalActorsToCueParams`)))

(event `self.AdditionalTargetDied`
  (params (DeadActor :type "Actor Object Reference"))
  ;[1 0.5176 0.1255] 额外目标敌人死亡
  ;;[1 1 1] 移除指定敌人的闪电链接
  (`self.RemoveShockLoopCuefromAdditionalTarget` DeadActor)
  (`KismetArrayLibrary.Array_RemoveItem` (`self. AdditionalTargets`) DeadActor))

(fn `AddShockLoopCueToAdditionalTarget`
  (params (AdditionalTarget :type "Actor Object Reference"))
  (locals (LocationTargetActor :type "Actor Object Reference"))
  (bind _locationtargetactor (`local.LocationTargetActor`))
  (bind _returnvalue (`AbilitySystemBlueprintLibrary.MakeGameplayCueParameters` 0.0 0.0 (struct) (struct) (struct) (struct) (struct) (`Actor.K2_GetActorLocation` _locationtargetactor) (0.0 0.0 0.0) null null _locationtargetactor null 1 1 (`Actor.RootComponent` (`self.MouseHitActor`))))
  (set `local.LocationTargetActor` AdditionalTarget)
  (`BlueprintMapLibrary.Map_Add` (`self.AdditionalActorsToCueParams`) (`local.LocationTargetActor`) _returnvalue)
  (`GameplayCueFunctionLibrary.AddGameplayCueOnActor` (`local.LocationTargetActor`) (struct :`TagName` "GameplayCue.ShockLoop") _returnvalue))

(fn `ApplyDamage`
  (`self.ApplyDamageSingleTarget` (`self.MouseHitActor`))
  (for _array_element (`self. AdditionalTargets`)
    (`self.ApplyDamageSingleTarget` _array_element)))

(fn `ApplyDamageSingleTarget`
  (params (Actor :type "Actor Object Reference"))
  (locals (LocalDamagedTarget :type "Actor Object Reference") (LocalASC :type "AbilitySystemComponent Object Reference"))
  (bind _returnvalue (`AbilitySystemBlueprintLibrary.GetAbilitySystemComponent` (`local.LocalDamagedTarget`)))
  (bind _output_get (set `local.LocalDamagedTarget` Actor))
  (`/Engine/EditorBlueprintResources/StandardMacros.IsValid` _output_get
    (:`Is Valid`
      (bind _output_get_2 (set `local.LocalASC` (`self.GetAbilitySystemComponentFromActorInfo`)))
      (`/Engine/EditorBlueprintResources/StandardMacros.IsValid` _output_get_2
        (:`Is Valid`
          (bind _returnvalue_2 (`AbilitySystemBlueprintLibrary.AssignTagSetByCallerMagnitude` (`AbilitySystemComponent.MakeOutgoingSpec` (`local.LocalASC`) (`self.DamageEffectClass`) (`KismetMathLibrary.Conv_IntToDouble` (`self.GetAbilityLevel`)) (`AbilitySystemComponent.MakeEffectContext` (`local.LocalASC`))) (struct :`TagName` "Damage.Lightning") (`self.GetDamageAtLevel`)))
          (`/Engine/EditorBlueprintResources/StandardMacros.IsValid` _returnvalue
            (:`Is Valid`
              (`AbilitySystemComponent.BP_ApplyGameplayEffectSpecToSelf` _returnvalue _returnvalue_2))))))))

(fn `ClearTimerAndEndAbility`
  (`KismetSystemLibrary.K2_ClearAndInvalidateTimerHandle` (`self.DamageAndCostTimer`))
  (`self.PrepareToEndAbility`)
  (`self.K2_CommitAbilityCooldown` false)
  (`KismetArrayLibrary.Array_Clear` (`self. AdditionalTargets`))
  (`BlueprintMapLibrary.Map_Clear` (`self.AdditionalActorsToCueParams`))
  (set `self.MouseHitActor` null)
  (set `self.FirstTargetImplementsInterface` false)
  (set `self.TimeHeld` 0.0)
  (`self.K2_EndAbility`))

(fn `EnforceImplementsCombatInterface`
  (if (not (`KismetSystemLibrary.DoesImplementInterface` (`self.GetAvatarActorFromActorInfo`) "/Script/Aura.CombatInterface"))
    (`self.K2_EndAbility`)))

(fn `InShockLoop`
  (message `CombatInterface.SetInShockLoop` (`self.GetAvatarActorFromActorInfo`) true)
  (`CharacterMovementComponent.DisableMovement` (`Character.CharacterMovement` (`self.OwnerCharacter`))))

(fn `PrepareToEndAbility`
  (bind _mousehitactor (`self.MouseHitActor`))
  (set `PlayerController.bShowMouseCursor` true (`self.OwnerPlayerController`))
  (message `CombatInterface.SetInShockLoop` (`self.GetAvatarActorFromActorInfo`) false)
  (`CharacterMovementComponent.SetMovementMode` (`Character.CharacterMovement` (`self.OwnerCharacter`)) "MOVE_Walking" 0)
  (if (`self.FirstTargetImplementsInterface`)
    (message `CombatInterface.SetIsBeingShocked` _mousehitactor false)
    (`GameplayCueFunctionLibrary.RemoveGameplayCueOnActor` _mousehitactor (struct :`TagName` "GameplayCue.ShockLoop") (`self.FirstTragetCueParams`))
    (`self.K2_HasAuthority`
      (:`True`
        (`AuraAbilitySystemLibrary.ApplyDamageEffect` (`self.MakeDamageEffectParamsFromClassDefaults` _mousehitactor)))
      (:`False`
        _))
    ;[1 1 1] 移除对应的额外敌人GC
    (for _array_element (`self. AdditionalTargets`)
      (message `CombatInterface.SetIsBeingShocked` _array_element false)
      (`self.RemoveShockLoopCuefromAdditionalTarget` _array_element)
      (`self.K2_HasAuthority`
        (:`True`
          (`AuraAbilitySystemLibrary.ApplyDamageEffect` (`self.MakeDamageEffectParamsFromClassDefaults` _array_element)))))
    (`BlueprintMapLibrary.Map_Clear` (`self.AdditionalActorsToCueParams`))
    (else
      (`GameplayCueFunctionLibrary.RemoveGameplayCueOnActor` (`self.GetAvatarActorFromActorInfo`) (struct :`TagName` "GameplayCue.ShockLoop") (`self.FirstTragetCueParams`)))))

(fn `RemoveShockLoopCuefromAdditionalTarget`
  (params (AdditionalTarget :type "Actor Object Reference"))
  (locals (LocalAddtionalTarget :type "Actor Object Reference"))
  (bind (_value _returnvalue) (`BlueprintMapLibrary.Map_Find` (`self.AdditionalActorsToCueParams`) (`local.LocalAddtionalTarget`)))
  (set `local.LocalAddtionalTarget` AdditionalTarget)
  (if _returnvalue
    (`GameplayCueFunctionLibrary.RemoveGameplayCueOnActor` (`local.LocalAddtionalTarget`) (struct :`TagName` "GameplayCue.ShockLoop") _value)))

(fn `SpawnElectricBeam`
  (locals (CueTarget :type "Actor Object Reference" :default null))
  ;[1 1 1] 第一个敌人
  (`self.TraceFirstTarget` (`self.MouseHitLocation`))
  (bind _returnvalue (message `CombatInterface.GetWeapon` (`self.GetAvatarActorFromActorInfo`)))
  (set `self.FirstTragetCueParams` (`AbilitySystemBlueprintLibrary.MakeGameplayCueParameters` 0.0 0.0 (struct) (struct) (struct) (struct) (struct) (`self.MouseHitLocation`) (0.0 0.0 0.0) null null (`self.MouseHitActor`) null 1 1 _returnvalue))
  ;[1 1 1] 第二个是否击中敌人
  (bind _output_get (set `self.FirstTargetImplementsInterface` (`KismetSystemLibrary.DoesImplementInterface` (`self.MouseHitActor`) "/Script/Aura.CombatInterface")))
  (if _output_get
    ;[1 1 1] 播放闪电特效和音效
    (set `local.CueTarget` (`self.MouseHitActor`))
    (else
      (set `local.CueTarget` (`self.GetAvatarActorFromActorInfo`))))
  (`GameplayCueFunctionLibrary.AddGameplayCueOnActor` (`local.CueTarget`) (struct :`TagName` "GameplayCue.ShockLoop") (`self.FirstTragetCueParams`))
  ;[1 1 1] 获取附近敌人
  (if (`self.FirstTargetImplementsInterface`)
    (message `CombatInterface.SetIsBeingShocked` (`local.CueTarget`) true)
    (bind _outadditionaltargets (`self.StoreAdditionalTargets`))
    (bind _output_get_2 (set `self. AdditionalTargets` _outadditionaltargets))
    (for _array_element _output_get_2
      (message `CombatInterface.SetIsBeingShocked` _array_element true)
      (`self.AddShockLoopCueToAdditionalTarget` _array_element))))

(fn `UpdateFacingTarget`
  (message `CombatInterface.UpdateFacingTarget` (`self.GetAvatarActorFromActorInfo`) (`self.MouseHitLocation`)))