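; Arcane Shards gameplay ability that erupts a level-scaled, capped number of shards around a ground point the player picks with a magic circle.
; On press, it spawns a BP_PointCollection for randomly rotated ground points, faces the target and plays the cast montage.
; The montage event commits cost and starts a looping timer that, per point, applies radial damage with outward knockback and fires a GameplayCue.
; Cooldown commits after the last shard.
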(event `self.K2_ActivateAbility`
  ;[1 1 1] 检查成本
  (bind _returnvalue (`self.K2_CheckAbilityCost`))
  (if _returnvalue
    (`|ExecutionSequence`
      (:`then_0`
        ;[1 1 1] 显示攻击范围
        (message `PlayerInterface.ShowMagicCircle` (`self.GetAvatarActorFromActorInfo`) null))
      (:`then_1`
        (`AbilityTask_WaitInputPress.WaitInputPress` false
          (:`OnPress`
            ;[1 1 1] 获取鼠标下目标数据
            (bind (_asynctaskproxy _datahandle) (`TargetDataUnderMouse.CreateTargetDataUnderMouse`)
              (:`ValidData`
                (set `self.MouseHitLocation` (`.ImpactPoint` (`GameplayStatics.BreakHitResult` (`AbilitySystemBlueprintLibrary.GetHitResultFromTargetData` _datahandle))))
                (`|ExecutionSequence`
                  (:`then_0`
                    ;[1 1 1] 生成点和获取要生成点的位置
                    (bind _returnvalue_2 (`|SpawnActorFromClass` "/Game/Blueprints/AbilitySystem/Aura/Abilities/Arcane/ArcaneShards/BP_PointCollection.BP_PointCollection_C" (`KismetMathLibrary.MakeTransform` (`self.MouseHitLocation`)) "AlwaysSpawn" "MultiplyWithRoot" null null))
                    (set `self.PointCollection` _returnvalue_2)
                    (set `self.NumShards` (`KismetMathLibrary.Min` (`self.MaxNumShards`) (`self.GetAbilityLevel`)))
                    (set `self.GroundPoints` (`PointCollection.GetGroundPoints` (`self.PointCollection`) (`self.MouseHitLocation`) (`self.NumShards`) (`KismetMathLibrary.RandomFloatInRange` 0.0 360.0))))
                  (:`then_1`
                    ;[1 1 1] 转向目标
                    (message `CombatInterface.UpdateFacingTarget` (`self.GetAvatarActorFromActorInfo`) (`self.MouseHitLocation`))
                    ;[1 1 1] 隐藏攻击范围
                    (message `PlayerInterface.HideMagicCircle` (`self.GetAvatarActorFromActorInfo`) null))
                  (:`then_2`
                    ;[1 1 1] 播放蒙太奇和等待事件
                    (`AbilityTask_PlayMontageAndWait.CreatePlayMontageAndWaitProxy` "None" "/Game/Assets/Characters/Aura/Animations/Abilities/AM_Cast_ArcaneShards.AM_Cast_ArcaneShards" 1.0 "None" false
                      (:`then`
                        (`AbilityTask_WaitGameplayEvent.WaitGameplayEvent` (struct :`TagName` "Event.Montage.ArcaneShards") null true
                          (:`EventReceived`
                            ;[1 1 1] 逐个生成点
                            (bind _returnvalue_3 (`KismetSystemLibrary.K2_SetTimerDelegate` (delegate `SpawnShard`) (`self.SpawnShardDeltaTime`) true))
                            (set `self.SpawnShardTimerHandle` _returnvalue_3)
                            (`self.SpawnShard`)
                            ;[1 1 1] 消耗蓝量
                            (`self.K2_CommitAbilityCost` false)))))))))))))
    (else
      (`self.K2_EndAbility`))))

(event `SpawnShard`
  ;[1 1 1] 逐个生成点
  (if (< (`self.Count`) (`self.NumShards`))
    (`self.StoreSpawnShardLocation`)
    ;[1 1 1] 应用伤害
    (`self.StorePlayersToDamage`)
    (for _array_element (`self.PlayersToDamage`)
      (`self.RadialDamageToPlayer` _array_element))
    (`/Engine/EditorBlueprintResources/StandardMacros.IncrementInt` (`self.Count`)
      (:`  `
        ;[1 1 1] GCN
        (`self.K2_ExecuteGameplayCueWithParams` (struct :`TagName` "GameplayCue.ArcaneShards") (`AbilitySystemBlueprintLibrary.MakeGameplayCueParameters` 0.0 0.0 (struct) (struct) (struct) (struct) (struct) (`self.SpawnShardLocation`)))))
    (else
      (`self.K2_EndAbility`)
      (`self.K2_CommitAbilityCooldown` false))))

(event `self.K2_OnEndAbility`
  (params (bWasCancelled :type Boolean))
  (bind _pointcollection (`self.PointCollection`)
    (:`then`
      (`Actor.K2_DestroyActor` _pointcollection)
      (`KismetSystemLibrary.K2_ClearAndInvalidateTimerHandle` (`self.SpawnShardTimerHandle`)))
    (:`else`)))

(fn `RadialDamageToPlayer`
  (params (TargetActor :type "Actor Object Reference"))
  (bind _returnvalue (- (`Actor.K2_GetActorLocation` TargetActor) (`self.SpawnShardLocation`)))
  (`AuraAbilitySystemLibrary.ApplyDamageEffect` (`self.MakeDamageEffectParamsFromClassDefaults` TargetActor (`self.SpawnShardLocation`) true _returnvalue true _returnvalue true 35.0)))

(fn `StorePlayersToDamage`
  (bind _returnvalue (`self.GetAvatarActorFromActorInfo`))
  (bind _outoverlappingactors (`AuraAbilitySystemLibrary.GetLivePlayerWithRadius` _returnvalue (`|MakeArray` _returnvalue) (`self.RadialDamageOuterRadius`) (`self.SpawnShardLocation`)))
  (set `self.PlayersToDamage` _outoverlappingactors))

(fn `StoreSpawnShardLocation`
  (set `self.SpawnShardLocation` (`SceneComponent.K2_GetComponentLocation` (`|GetArrayItem` (`self.GroundPoints`) (`self.Count`)))))