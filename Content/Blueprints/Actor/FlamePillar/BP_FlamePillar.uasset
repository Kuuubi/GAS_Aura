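; BP_FlamePillar is a flame pillar actor that makes its FireLight flicker continuously from BeginPlay.
; It randomly picks one of two timelines, each driving the light's intensity as a curve value multiplied by BaseIntensity.
; When a timeline finishes it triggers a new random pick, chaining the two curves into an endless, varied flicker without using Tick.
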(event `self.ReceiveBeginPlay`
  (`self.ChooseTimeline`))

(event `ChooseTimeline`
  ;[1 1 1] 火光强度
  (switch `int` (`KismetMathLibrary.RandomIntegerInRange` 0 1)
    (:`Default`
      (`self.StartTimeline_2` :!label _label))
    (:`0`
      (`self.StartTimeline_1`))
    (:`1`
      (goto _label))))

(event `StartTimeline_1`
  ;[1 1 1] 火光强度
  (bind (_direction _flameintensity_1) (`Timeline|FlameIntensity_1` :!via `PlayFromStart`)
    (:`Update`
      (`LightComponent.SetIntensity` (`self.FireLight`) (* _flameintensity_1 (`self.BaseIntensity`))))
    (:`Finished`
      (`self.ChooseTimeline`))))

(event `StartTimeline_2`
  ;[1 1 1] 火光强度
  (bind (_direction _flameintensity_2) (`Timeline|FlameIntensity_2` :!via `PlayFromStart`)
    (:`Update`
      (`LightComponent.SetIntensity` (`self.FireLight`) (* _flameintensity_2 (`self.BaseIntensity`))))
    (:`Finished`
      (`self.ChooseTimeline`))))

(fn `UserConstructionScript`)